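; Collectable resource node that a ColonyCharacter harvests to grow its bacteria colony, configured through a Construct event with randomized stock.
; On Tick, an overlapping colony meeting the minimum size triggers timed harvests, each spending one unit to create a random number of bacteria.
; Larger colonies shorten the cooldown between harvests, and the actor destroys itself once found empty.
; Collection sphere overlap events toggle the colony's Busy flag.
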(event OnComponentBeginOverlap(SphereCollect)
  (params (OverlappedComponent :type Primitive%20Component%20Object%20Reference) (OtherActor :type Actor%20Object%20Reference) (OtherComp :type Primitive%20Component%20Object%20Reference) (OtherBodyIndex :type Integer) (bFromSweep :type Boolean) (SweepResult :type Hit%20Result%20Structure%20%28by%20ref%29))
  (bind _ascolony_character (Utilities|Casting|CastToColonyCharacter OtherActor))
  (Variables|/Game/Colony/ColonyCharacter.ColonyCharacter_C|SetBusy _ascolony_character true))

(event OnComponentEndOverlap(SphereCollect)
  (params (OverlappedComponent :type Primitive%20Component%20Object%20Reference) (OtherActor :type Actor%20Object%20Reference) (OtherComp :type Primitive%20Component%20Object%20Reference) (OtherBodyIndex :type Integer))
  (bind _ascolony_character (Utilities|Casting|CastToColonyCharacter OtherActor))
  (Variables|/Game/Colony/ColonyCharacter.ColonyCharacter_C|SetBusy _ascolony_character false))

(event Custom|Construct
  (params (CD :type Float%20%28single-precision%29) (minEnt :type Integer) (minRes :type Integer) (maxRes :type Integer) (Nbmin :type Integer) (Nbmax :type Integer))
  (Variables|Default|SetDefaultCD CD)
  (Variables|Default|SetCoolDown CD)
  (Variables|Default|SetminEnt minEnt)
  (Variables|Default|SetRes (Math|Random|RandomIntegerinRange minRes maxRes))
  (Variables|Default|SetNbmin Nbmin)
  (Variables|Default|SetNbmax Nbmax))

(event EventBeginPlay)

(event EventTick
  (params (DeltaSeconds :type Float%20%28single-precision%29))
  (bind _spherecollect (Variables|Default|GetSphereCollect))
  (bind _overlappingactors (Collision|GetOverlappingActors _spherecollect "/Game/Colony/ColonyCharacter.ColonyCharacter_C" :!class /Script/Engine.PrimitiveComponent))
  (bind _output (Utilities|Array|Get(acopy) _overlappingactors))
  (bind _ascolony_character (Utilities|Casting|CastToColonyCharacter _output))
  (if (>= (Utilities|Array|Length (Variables|/Game/Colony/ColonyCharacter.ColonyCharacter_C|GetBacterias _ascolony_character)) (Variables|Default|GetminEnt))
    (Variables|Default|SetCurrentCD (- (Variables|Default|GetDefaultCD) (* (Math|Conversions|ToFloat(Integer) (Utilities|Array|Length (Variables|/Game/Colony/ColonyCharacter.ColonyCharacter_C|GetBacterias _ascolony_character))) 0.05)))
    (if (> (Variables|Default|GetRes) 0)
      (if (<= (Variables|Default|GetCoolDown) 0.0)
        (bind _ascolony_character_2 (Utilities|Casting|CastToColonyCharacter _output))
        (Default|CreateBacteria _ascolony_character_2 (Math|Random|RandomIntegerinRange (Variables|Default|GetNbmin) (Variables|Default|GetNbmax)))
        (Math|Integer|DecrementInt (Variables|Default|GetRes)
          (:%20%20
            (Variables|Default|SetCoolDown (Variables|Default|GetCurrentCD))))
        (else
          (Variables|Default|SetCoolDown (- (Variables|Default|GetCoolDown) DeltaSeconds))))
      (else
        (Actor|DestroyActor)))))

(fn ConstructionScript)