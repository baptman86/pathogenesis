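; CollectableCells_BP is a collectable cell actor that lights up when a bacteria first reaches it.
; On BeginPlay it calls Construct with entity and resource limits and creates a dynamic instance of the highlighted blood vessel material on its mesh.
; When a Bacteria_AI first overlaps the SphereCollect component, it raises the material's Emissive parameter, with a MatSet flag preventing repeats.
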(event OnComponentBeginOverlap(SphereCollect)
  (params (OverlappedComponent :type Primitive%20Component%20Object%20Reference) (OtherActor :type Actor%20Object%20Reference) (OtherComp :type Primitive%20Component%20Object%20Reference) (OtherBodyIndex :type Integer) (bFromSweep :type Boolean) (SweepResult :type Hit%20Result%20Structure%20%28by%20ref%29))
  (if (not (Variables|Default|GetMatSet))
    (Utilities|Casting|CastToBacteria_AI OtherActor)
    (Rendering|Material|SetScalarParameterValue (Variables|Default|GetMat) "Emissive" 1.0 :!class /Script/Engine.MaterialInstanceDynamic)
    (Variables|Default|SetMatSet true)))

(event EventBeginPlay
  (CallFunction|Construct 6.0 10 5 15 1 5)
  (bind _returnvalue (Rendering|Material|CreateDynamicMaterialInstance (Variables|Character|GetMesh) 0 "/Game/StarterContent/Materials/BloodVesselHighlighted_Mat.BloodVesselHighlighted_Mat" "None" :!class /Script/Engine.PrimitiveComponent))
  (Variables|Default|SetMat _returnvalue))

(event Collision|EventActorBeginOverlap
  (params (OtherActor :type Actor%20Object%20Reference)))

(event EventTick
  (params (DeltaSeconds :type Float%20%28single-precision%29)))

(fn ConstructionScript
  (|CallParentFunction))