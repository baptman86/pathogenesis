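; Top-down camera Blueprint that pans and zooms the view and can recenter it on a colony.
; After binding UI_Schema's edge widgets and centering the mouse following a start delay, Tick feeds movement offsets to the camera.
; Edge hover pans after a cooldown with acceleration, while directional input flags pan immediately.
; Zoom steps between two height limits, drifting toward the cursor on wheel zoom-in, and pans faster when zoomed out.
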(event Custom|CenterCameraOnColony
  (params (X :type Float%20%28single-precision%29) (Y :type Float%20%28single-precision%29))
  (bind _cameracomponent (Variables|CameraActor|GetCameraComponent))
  (Transformation|SetWorldLocation _cameracomponent (Math|Vector|MakeVector X Y (.z (Transformation|GetWorldLocation _cameracomponent))) false true))

(event EventTick
  (params (DeltaSeconds :type Float%20%28single-precision%29))
  (bind _cooldown (Variables|Default|GetCoolDown))
  (if (Variables|Default|GetisInit)
    (if (> (Variables|Default|Getwait%20start) 0)
      (CallFunction|WaittoStart)
      (elif (== (Variables|Default|GetZoomMode) 0)
        (if (Variables|Default|GetCanZoom)
          (bind _dozoom (CallFunction|ComputeZoom))
          (if (not _dozoom)
            (bind _move (CallFunction|MoveCompute :!label _label))
            (if _move
              (if (<= _cooldown 0)
                (Transformation|AddRelativeLocation (Variables|CameraActor|GetCameraComponent) (Math|Vector|MakeVector (Variables|Default|GetFinalXCoeff) (Variables|Default|GetFinalYCoeff) (Variables|Default|GetFinalZCoeff)) false false :!label _label_2)
                (else
                  (Math|Integer|DecrementInt _cooldown)))))
          (else
            (goto _label)))
        (else
          (bind _finished (CallFunction|DoZoom))
          (if _finished
            (goto _label)
            (else
              (goto _label_2))))))
    (else
      (bind _success (CallFunction|Init))
      (Variables|Default|SetisInit _success))))

(fn ConstructionScript)

(fn WaittoStart
  (bind _returnvalue (Viewport|GetViewportSize))
  (bind (_x _y) (Math|Vector2D|BreakVector2D _returnvalue))
  (Math|Integer|DecrementInt (Variables|Default|Getwait%20start)
    (:%20%20
      (if (<= (Variables|Default|Getwait%20start) 0)
        (Class|PlayerController|SetMouseLocation (Game|GetPlayerController 0) (Math|Float|Truncate (/ _x 2.0)) (Math|Float|Truncate (/ _y 2.0)))
        (Variables|Default|Setwait%20start 0)
        (return)))))

(fn ComputeZoom
  (bind _zmax (Variables|Default|GetZmax))
  (bind _zmin (Variables|Default|GetZmin))
  (bind _zoomcoeffz (Variables|Default|GetZoomCoeffZ))
  (bind _cameracomponent (Variables|CameraActor|GetCameraComponent))
  (bind _returnvalue (Transformation|GetWorldLocation _cameracomponent))
  (bind _returnvalue_2 (- _zmax _zmin))
  (bind _astop_down_character (Utilities|Casting|CastToTopDownCharacter (Game|GetPlayerCharacter 0)))
  (if (or (and (Variables|Default|GetToggleZoom) (== (Variables|Default|GetCameraZoom) 0)) (Variables|Default|GetGotWheelUp))
    (Variables|Default|SetGotWheelUp false)
    (Variables|Default|SetZoomMode 1)
    (Variables|Default|SetCameraZoom 1)
    (Variables|Default|SetMoveCoeffZoomMult 1.0)
    (elif (or (and (Variables|Default|GetToggleZoom) (== (Variables|Default|GetCameraZoom) 1)) (Variables|Default|GetGotWheelDown))
      (Variables|Default|SetGotWheelDown false)
      (Variables|Default|SetZoomMode 2)
      (Variables|Default|SetCameraZoom 0)
      (Variables|Default|SetMoveCoeffZoomMult 6.0)
      (else
        (return false))))
  (if (Variables|Default|GetToggleZoom)
    (Variables|Default|SetToggleZoom false)
    (Variables|Default|SetZoomCoeffX 0.0)
    (Variables|Default|SetZoomCoeffY 0.0)
    (else
      (Variables|Default|SetZoomCoeffX (* (/ (- (.x (Transformation|GetWorldLocation (Variables|/Game/TopDownBP/Blueprints/TopDownCharacter.TopDownCharacter_C|GetCursorToWorld _astop_down_character))) (.x _returnvalue)) _returnvalue_2) _zoomcoeffz))
      (Variables|Default|SetZoomCoeffY (* (/ (- (.y (Transformation|GetWorldLocation (Variables|/Game/TopDownBP/Blueprints/TopDownCharacter.TopDownCharacter_C|GetCursorToWorld _astop_down_character))) (.y _returnvalue)) _returnvalue_2) _zoomcoeffz))))
  (return true))

(fn DoZoom
  (bind _cameracomponent (Variables|CameraActor|GetCameraComponent))
  (bind _returnvalue (Transformation|GetWorldLocation _cameracomponent))
  (if (and (== (Variables|Default|GetZoomMode) 1) (<= (Variables|Default|GetZmin) (.z _returnvalue)))
    (Variables|Default|SetFinalXCoeff (Variables|Default|GetZoomCoeffX))
    (Variables|Default|SetFinalYCoeff (Variables|Default|GetZoomCoeffY))
    (Variables|Default|SetFinalZCoeff (* (Variables|Default|GetZoomCoeffZ) -1.0))
    (elif (and (== (Variables|Default|GetZoomMode) 2) (>= (Variables|Default|GetZmax) (.z _returnvalue)))
      (Variables|Default|SetFinalXCoeff 0.0)
      (Variables|Default|SetFinalYCoeff 0.0)
      (Variables|Default|SetFinalZCoeff (Variables|Default|GetZoomCoeffZ))
      (else
        (Variables|Default|SetZoomMode 0)
        (return true))))
  (return false))

(fn MoveCompute
  (bind _topright (Variables|Default|GetTopRight))
  (bind _topleft (Variables|Default|GetTopLeft))
  (bind _bottomright (Variables|Default|GetBottomRight))
  (bind _bottomleft (Variables|Default|GetBottomLeft))
  (bind _right (Variables|Default|GetRight))
  (bind _right_2 (Variables|Default|GetRight))
  (bind _gotright (Variables|Default|GetGotRight))
  (bind _gotleft (Variables|Default|GetGotLeft))
  (bind _gottop (Variables|Default|GetGotTop))
  (bind _left (Variables|Default|GetLeft))
  (bind _gotbottom (Variables|Default|GetGotBottom))
  (bind _top (Variables|Default|GetTop))
  (bind _bottom (Variables|Default|GetBottom))
  (Widget|SetRenderOpacity _right 0.0)
  (if (Math|Boolean|ORBoolean (Widget|IsHovered _right) (Widget|IsHovered (Variables|Default|GetLeft)) (Widget|IsHovered (Variables|Default|GetTop)) (Widget|IsHovered (Variables|Default|GetBottom)) (Widget|IsHovered (Variables|Default|GetTopRight)) (Widget|IsHovered (Variables|Default|GetTopLeft)) (Widget|IsHovered (Variables|Default|GetBottomRight)) (Widget|IsHovered (Variables|Default|GetBottomLeft)))
    (Variables|Default|SetFinalXCoeff 0.0 :!label _label)
    (Variables|Default|SetFinalYCoeff 0.0)
    (Variables|Default|SetFinalZCoeff 0.0)
    (if (or (Widget|IsHovered _topright) (and _gotright _gottop)) ; isTopRight
      (Widget|SetRenderOpacity _topright 1.0)
      ;[1 1 1] TopRight
      (Variables|Default|SetFinalXCoeff (* (Variables|Default|GetMoveCoeffZoomMult) (Variables|Default|GetMoveCoeff))) ; x = c
      (Variables|Default|SetFinalYCoeff (* (Variables|Default|GetMoveCoeffZoomMult) (Variables|Default|GetMoveCoeff))) ; y = c
      (elif (or (Widget|IsHovered _bottomright) (and _gotright _gotbottom)) ; isBottomRight
        (Widget|SetRenderOpacity _bottomright 1.0)
        ;[1 1 1] BottomRight
        (Variables|Default|SetFinalXCoeff (* (* (Variables|Default|GetMoveCoeffZoomMult) (Variables|Default|GetMoveCoeff)) -1.0)) ; x = -c
        (Variables|Default|SetFinalYCoeff (* (Variables|Default|GetMoveCoeffZoomMult) (Variables|Default|GetMoveCoeff))) ; y = c
        (elif (or (Widget|IsHovered _right_2) _gotright) ; isRight
          ;[1 1 1] Calc Coeff
          (Widget|SetRenderOpacity _right_2 1.0)
          ;[1 1 1] Right
          (Variables|Default|SetFinalYCoeff (* (* (Variables|Default|GetMoveCoeffZoomMult) (Variables|Default|GetMoveCoeff)) 1.25)) ; Y = 1.25c
          (elif (or (Widget|IsHovered _topleft) (and _gotleft _gottop)) ; isTopLeft
            (Widget|SetRenderOpacity _topleft 1.0)
            ;[1 1 1] TopLeft
            (Variables|Default|SetFinalXCoeff (* (Variables|Default|GetMoveCoeffZoomMult) (Variables|Default|GetMoveCoeff))) ; x = c
            (Variables|Default|SetFinalYCoeff (* (* (Variables|Default|GetMoveCoeffZoomMult) (Variables|Default|GetMoveCoeff)) -1.0)) ; y = -c
            (elif (or (Widget|IsHovered _bottomleft) (and _gotleft _gotbottom)) ; isBottomLeft
              (Widget|SetRenderOpacity _bottomleft 1.0)
              ;[1 1 1] BottomLeft
              (Variables|Default|SetFinalXCoeff (* (* (Variables|Default|GetMoveCoeffZoomMult) (Variables|Default|GetMoveCoeff)) -1.0)) ; x = -c
              (Variables|Default|SetFinalYCoeff (* (* (Variables|Default|GetMoveCoeffZoomMult) (Variables|Default|GetMoveCoeff)) -1.0)) ; y = -c
              (elif (or (Widget|IsHovered _left) _gotleft) ; isLeft
                (Widget|SetRenderOpacity _left 1.0)
                ;[1 1 1] Left
                (Variables|Default|SetFinalYCoeff (* (* (* (Variables|Default|GetMoveCoeffZoomMult) (Variables|Default|GetMoveCoeff)) 1.25) -1.0)) ; Y = -1.25c
                (elif (or (Widget|IsHovered _top) _gottop) ; isTop
                  (Widget|SetRenderOpacity _top 1.0)
                  ;[1 1 1] Top
                  (Variables|Default|SetFinalXCoeff (* (* (Variables|Default|GetMoveCoeffZoomMult) (Variables|Default|GetMoveCoeff)) 1.25)) ; X = 1.25c
                  (elif (or (Widget|IsHovered _bottom) _gotbottom) ; isBottom
                    (Widget|SetRenderOpacity _bottom 1.0)
                    ;[1 1 1] Bottom
                    (Variables|Default|SetFinalXCoeff (* (* (* (Variables|Default|GetMoveCoeffZoomMult) (Variables|Default|GetMoveCoeff)) 1.25) -1.0)) ; X = -1.25c
                    (else
                      ;[1 1 1] Reset Coeff and CD
                      (Variables|Default|SetMoveCoeff (Variables|Default|GetMinMoveCoeff) :!label _label_2)
                      (Variables|Default|SetCoolDown (Variables|Default|GetDefaultCD))
                      (return false))))))))))
    (else
      (Variables|Default|SetCoolDown 0)
      (Variables|Default|SetMoveCoeff (Variables|Default|GetMoveCoeffMax))
      (if (Math|Boolean|ORBoolean _gotright _gotleft _gottop _gotbottom)
        (goto _label)
        (else
          (goto _label_2)))))
  ;[1 1 1] Inc Coeff
  (if (<= (Variables|Default|GetMoveCoeff) (+ (Variables|Default|GetMoveCoeffMax) (* (- (Variables|Default|GetMoveCoeffZoomMult) 1.0) 2.0)))
    (Variables|Default|SetMoveCoeff (* (Variables|Default|GetMoveCoeff) 1.05)))
  (return true))

(fn Init
  (bind _foundwidgets (Widget|GetAllWidgetsOfClass "/Game/UI/UI_Schema.UI_Schema_C" false))
  (if (> (Utilities|Array|Length _foundwidgets) 0)
    (Variables|Default|SetRight (Variables|/Game/UI/UI_Schema.UI_Schema_C|GetRight (Utilities|Array|Get(acopy) _foundwidgets)))
    (Variables|Default|SetLeft (Variables|/Game/UI/UI_Schema.UI_Schema_C|GetLeft (Utilities|Array|Get(acopy) _foundwidgets)))
    (Variables|Default|SetTop (Variables|/Game/UI/UI_Schema.UI_Schema_C|GetTop (Utilities|Array|Get(acopy) _foundwidgets)))
    (Variables|Default|SetBottom (Variables|/Game/UI/UI_Schema.UI_Schema_C|GetBottom (Utilities|Array|Get(acopy) _foundwidgets)))
    (Variables|Default|SetTopRight (Variables|/Game/UI/UI_Schema.UI_Schema_C|GetTopRight (Utilities|Array|Get(acopy) _foundwidgets)))
    (Variables|Default|SetTopLeft (Variables|/Game/UI/UI_Schema.UI_Schema_C|GetTopLeft (Utilities|Array|Get(acopy) _foundwidgets)))
    (Variables|Default|SetBottomRight (Variables|/Game/UI/UI_Schema.UI_Schema_C|GetBottomRight (Utilities|Array|Get(acopy) _foundwidgets)))
    (Variables|Default|SetBottomLeft (Variables|/Game/UI/UI_Schema.UI_Schema_C|GetBottomLeft (Utilities|Array|Get(acopy) _foundwidgets)))
    (return true)
    (else
      (return false))))